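; BP_TemporalLobe is a brain-section trigger that relocates the third-person character when it enters or leaves its box.
; Each overlap moves the character to the stored NewLocation and saves the previous position there through ChangeLocation, so the destination alternates.
; It also sets FlipControlsActive on entry and clears it on exit, though nothing in this Blueprint reads that flag.
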(event `self.Box.OnComponentBeginOverlap`
  (params (OverlappedComponent :type "PrimitiveComponent Object Reference") (OtherActor :type "Actor Object Reference") (OtherComp :type "PrimitiveComponent Object Reference") (OtherBodyIndex :type Integer) (bFromSweep :type Boolean) (SweepResult :type "HitResult Structure (by ref)"))
  (bind _asbp_third_person_character (cast `/Game/ThirdPersonBP/Blueprints/BP_ThirdPersonCharacter` OtherActor))
  (set `self.Flip Controls Active` true)
  (bind _output_get (set `self.ChangeLocation` (`/Game/ThirdPersonBP/Blueprints/BP_ThirdPersonCharacter.Location` _asbp_third_person_character)))
  (set `/Game/ThirdPersonBP/Blueprints/BP_ThirdPersonCharacter.Location` (`self.NewLocation`) _asbp_third_person_character)
  (set `self.NewLocation` _output_get))

(event `self.Box.OnComponentEndOverlap`
  (params (OverlappedComponent :type "PrimitiveComponent Object Reference") (OtherActor :type "Actor Object Reference") (OtherComp :type "PrimitiveComponent Object Reference") (OtherBodyIndex :type Integer))
  (bind _asbp_third_person_character (cast `/Game/ThirdPersonBP/Blueprints/BP_ThirdPersonCharacter` OtherActor))
  (set `self.Flip Controls Active` false)
  (bind _output_get (set `self.ChangeLocation` (`/Game/ThirdPersonBP/Blueprints/BP_ThirdPersonCharacter.Location` _asbp_third_person_character)))
  (set `/Game/ThirdPersonBP/Blueprints/BP_ThirdPersonCharacter.Location` (`self.NewLocation`) _asbp_third_person_character)
  (set `self.NewLocation` _output_get))

(fn `UserConstructionScript`)