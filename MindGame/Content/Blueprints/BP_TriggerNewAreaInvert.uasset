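; Trigger volume that inverts the third-person character's controls while it is inside the collision box.
; Begin overlap caches the character, sets its FlipControls and swaps its Location value with CerebellumLocation.
; End overlap swaps the values back before its cast check, then waits three seconds and copies ControlsFlipped to the character, so re-entering during the delay keeps controls inverted.
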(event `self.CollisionBox.OnComponentBeginOverlap`
  (params (OverlappedComponent :type "PrimitiveComponent Object Reference") (OtherActor :type "Actor Object Reference") (OtherComp :type "PrimitiveComponent Object Reference") (OtherBodyIndex :type Integer) (bFromSweep :type Boolean) (SweepResult :type "HitResult Structure (by ref)"))
  (set `self.ControlsFlipped` true)
  (bind _asbp_third_person_character (cast `/Game/ThirdPersonBP/Blueprints/BP_ThirdPersonCharacter` OtherActor))
  (bind _output_get (set `self.CharacterREF` _asbp_third_person_character))
  (set `/Game/ThirdPersonBP/Blueprints/BP_ThirdPersonCharacter.FlipControls` true _output_get)
  (set `self.ControlsFlipped` true)
  (bind _output_get_2 (set `self.ChangeLocation` (`/Game/ThirdPersonBP/Blueprints/BP_ThirdPersonCharacter.Location` _asbp_third_person_character)))
  (set `/Game/ThirdPersonBP/Blueprints/BP_ThirdPersonCharacter.Location` (`self.CerebellumLocation`) _asbp_third_person_character)
  (set `self.CerebellumLocation` _output_get_2))

(event `self.CollisionBox.OnComponentEndOverlap`
  (params (OverlappedComponent :type "PrimitiveComponent Object Reference") (OtherActor :type "Actor Object Reference") (OtherComp :type "PrimitiveComponent Object Reference") (OtherBodyIndex :type Integer))
  (set `self.ControlsFlipped` false)
  (bind _output_get (set `self.ChangeLocation` (`/Game/ThirdPersonBP/Blueprints/BP_ThirdPersonCharacter.Location` (`self.CharacterREF`))))
  (set `/Game/ThirdPersonBP/Blueprints/BP_ThirdPersonCharacter.Location` (`self.CerebellumLocation`) (`self.CharacterREF`))
  (set `self.CerebellumLocation` _output_get)
  (cast `/Game/ThirdPersonBP/Blueprints/BP_ThirdPersonCharacter` OtherActor)
  (`KismetSystemLibrary.Delay` 3.0)
  (if (== (`self.ControlsFlipped`) true)
    (set `/Game/ThirdPersonBP/Blueprints/BP_ThirdPersonCharacter.FlipControls` true (`self.CharacterREF`))
    (else
      (set `/Game/ThirdPersonBP/Blueprints/BP_ThirdPersonCharacter.FlipControls` false (`self.CharacterREF`)))))

(fn `UserConstructionScript`)