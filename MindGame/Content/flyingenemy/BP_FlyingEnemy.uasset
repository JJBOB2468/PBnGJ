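; Flying enemy pawn that targets the first player character it sees through PawnSensing, then chases or circles it.
; Tick, gated by a Location equality check against the player, approaches outside AttackRange and strafes within it, smoothing rotation toward the target.
; A randomized, self-restarting timer alternates strafe direction.
; Within range it also calls LeapAttack for a forward lunge; the delayed CanAttack reset does not gate that call.
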(event `self.ReceiveBeginPlay`
  (`self.Change Strafe direction`))

(event `Change Strafe direction`
  (bind _isa (`/Engine/EditorBlueprintResources/StandardMacros.FlipFlop`)
    (:`A`
      _)
    (:`B`
      _))
  (set `self.strive right` _isa)
  (`KismetSystemLibrary.K2_SetTimerDelegate` (delegate `Change Strafe direction`) (`KismetMathLibrary.RandomFloatInRange` 2.0 6.0)))

(event `self.ReceiveTick`
  (params (DeltaSeconds :type "Float (single-precision)"))
  (bind _returnvalue (`self.K2_GetActorLocation`))
  (bind _asbp_third_person_character (cast `/Game/ThirdPersonBP/Blueprints/BP_ThirdPersonCharacter` (`GameplayStatics.GetPlayerCharacter` 0)))
  (if (== (`self.Location`) (`/Game/ThirdPersonBP/Blueprints/BP_ThirdPersonCharacter.Location` _asbp_third_person_character))
    (bind _target (`self.Target`)
      (:`then`
        (if (> (`self.GetDistanceTo` _target) (`self.AttackRange`))
          (bind _returnvalue_2 (`self.K2_GetActorLocation` _target))
          (bind (_returnvalue_roll _returnvalue_pitch _returnvalue_yaw) (`KismetMathLibrary.BreakRotator` (`KismetMathLibrary.FindLookAtRotation` _returnvalue (+ _returnvalue_2 (0.0 0.0 100.0)))))
          (`self.AddMovementInput` (`KismetMathLibrary.Conv_RotatorToVector` (`KismetMathLibrary.MakeRotator` 0.0 0.0 _returnvalue_yaw)))
          (`self.K2_SetActorRotation` (`KismetMathLibrary.RLerp` (`self.K2_GetActorRotation`) (`KismetMathLibrary.MakeRotator` 0.0 0.0 _returnvalue_yaw) 0.1 true))
          (else
            (bind _returnvalue_3 (`KismetMathLibrary.FindLookAtRotation` _returnvalue _returnvalue_2))
            (`self.AddMovementInput` (`KismetMathLibrary.GetRightVector` _returnvalue_3) (`KismetMathLibrary.SelectFloat` 0.5 -0.5 (`self.strive right`)))
            (`self.K2_SetActorRotation` (`KismetMathLibrary.RLerp` (`self.K2_GetActorRotation`) _returnvalue_3 0.1 true))
            (if (`self.CanAttack`)
              _
              (else
                _))
            (`self.LeapAttack`)
            (set `self.CanAttack` false)
            (`KismetSystemLibrary.Delay` 10.0)
            (set `self.CanAttack` true))))
      (:`else`))))

(event `self.PawnSensing.OnSeePawn`
  (params (Pawn :type "Pawn Object Reference"))
  (`self.Target`
    (:`then`)
    (:`else`
      (bind _asbp_third_person_character (cast `/Game/ThirdPersonBP/Blueprints/BP_ThirdPersonCharacter` Pawn))
      (set `self.Target` _asbp_third_person_character))))

(event `LeapAttack`
  (bind _charactermovement (`self.CharacterMovement`))
  (bind _returnvalue (* (`KismetMathLibrary.GetForwardVector` (`self.K2_GetActorRotation`)) (60.0 60.0 0.0)))
  (`CharacterMovementComponent.AddImpulse` _charactermovement _returnvalue true)
  (`CharacterMovementComponent.AddForce` _charactermovement _returnvalue)
  (set `self.CanAttack` false))

(fn `UserConstructionScript`)