(event `self.ReceiveTick`
  (params (DeltaSeconds :type "Float (single-precision)"))
  (set `self.attackWait` (+ (`self.attackWait`) DeltaSeconds))
  (`self.follow player`)
  (if (`self.CanAttack`)
    (set `self.CanAttack` false)
    (`self.LeapAttack`)
    (else
      (`KismetSystemLibrary.Delay` 2.0)
      (set `self.CanAttack` true))))

(event `self.PawnSensing.OnSeePawn`
  (params (Pawn :type "Pawn Object Reference"))
  (bind _asbp_third_person_character (cast `/Game/ThirdPersonBP/Blueprints/BP_ThirdPersonCharacter` Pawn))
  (set `self.target` _asbp_third_person_character))

(event `follow player`
  (if (>= (`self.GetDistanceTo` (`self.target`)) 0.0)
    (`|AIMoveTo` self (0.0 0.0 0.0) (`self.target`) 0.0 true
      (:`then`
        _))
    (else
      (`|AIMoveTo` self (0.0 0.0 0.0) self
        (:`then`
          _))))
  (`KismetSystemLibrary.Delay` 0.2)
  (`self.follow player`))

(event `LeapAttack`
  (bind _charactermovement (`self.CharacterMovement`))
  (bind _target (`self.Target`))
  (bind _returnvalue (* (`KismetMathLibrary.GetForwardVector` (`self.K2_GetActorRotation`)) (1000.0 1000.0 0.0)))
  (`CharacterMovementComponent.AddImpulse` _charactermovement _returnvalue true)
  (`CharacterMovementComponent.AddForce` _charactermovement _returnvalue)
  (if (`self.IsOverlappingActor` (`self.Target`))
    (if (> (`self.attackWait`) 1.0)
      (set `/Game/ThirdPersonBP/Blueprints/BP_ThirdPersonCharacter.Health` (- (`/Game/ThirdPersonBP/Blueprints/BP_ThirdPersonCharacter.Health` _target) 1) _target)
      (set `self.CanAttack` false)
      (set `self.attackWait` 0.0))
    (else
      (set `self.CanAttack` false))))

(fn `Change Strafe direction`)

(fn `UserConstructionScript`)